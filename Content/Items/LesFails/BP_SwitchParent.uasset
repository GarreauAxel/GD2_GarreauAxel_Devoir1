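; Parent Blueprint for switches that open doors when interacted with.
; Interaction calls Opening, which sends YesMessage to each entry in an Actor array that implements the BPI_doors interface.
; A separate OpenDoor event, not called in this graph, uses Checking to match each BPDoor's DoorNumber against the switch's DoorsNumber list, then calls Opening on matches and prints debug text.
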(event Custom|OpenDoor
  ;[1 0 0.1318] Un code qui permet de dire quel interrupteur ouvre quelle porte avec un système d'integer, le problème étant qu'il faut passer une variable d'un blueprint a un autre et j'ai pas trouvé comment faire sans get actor of class (ce qui m'aurais value une mauvaise note) donc si il existe un moyen de faire ça plus proprement ça serais interressant
  (for _array_element (Variables|Default|GetBP_door)
    (bind (_output_get _doortoopen) (CallFunction|Checking (Variables|/Game/Items/BP_DoorParent.BP_DoorParent_C|GetDoorNumber _array_element) _array_element))
    (if _output_get
      (Development|PrintString "great i found you")
      (Default|Opening _doortoopen)
      (else
        (Development|PrintString "404 not found")))))

(event Custom|Opening
  ;[1 1 1] interface système
  (for _array_element (Variables|Default|GetActor)
    (if (Utilities|DoesObjectImplementInterface _array_element "/Game/Items/Blueprint/BPI_doors.BPI_doors_C")
      (Class|BPIDoors|Yes(Message) _array_element))))

(event EventBeginPlay)

(event Collision|EventActorBeginOverlap
  (params (OtherActor :type Actor%20Object%20Reference)))

(event EventTick
  (params (DeltaSeconds :type Float%20%28single-precision%29)))

(event EventInteraction
  (CallFunction|Opening))

(fn ConstructionScript)

(fn Checking
  (params (DoorIdentity :type Integer) (DoorWhoOpen :type BP%20Door%20Parent%20Object%20Reference))
  (for _array_element (Variables|Default|GetDoorsNumber)
    (if (== DoorIdentity _array_element)
      (bind _output_get (Variables|Default|SetOpen true))
      (return _output_get DoorWhoOpen))))