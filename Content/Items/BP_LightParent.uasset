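; BP_LightParent is a parent light actor that turns on when the required number of doors is open.
; AddOne and LessOne events raise or lower an open-door Count, then call Checking.
; Checking shows the PointLight only when Count exactly equals GoodCount and hides it otherwise, so extra open doors also switch it off.
; It does not poll on Tick, and visibility updates only when one of those events is called.
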(event EventBeginPlay)

(event Collision|EventActorBeginOverlap
  (params (OtherActor :type Actor%20Object%20Reference)))

(event EventTick
  (params (DeltaSeconds :type Float%20%28single-precision%29)))

(event EventAddOne
  ;[1 1 1] Système d'integer pour savoir combien de portes sont ouverte
  (Variables|Default|SetCount (+ (Variables|Default|GetCount) 1))
  (CallFunction|Checking))

(event EventLessOne
  ;[1 1 1] Système d'integer pour savoir combien de portes sont ouverte
  (Variables|Default|SetCount (+ (Variables|Default|GetCount) -1))
  (CallFunction|Checking))

(fn ConstructionScript)

(fn Checking
  (bind _pointlight (Variables|Default|GetPointLight))
  ;[1 1 1] Vérifier que le nombre de portes ouvertes corresponde bien au nombre de porte qui doivent l'être pour allumer la lumière
  (if (== (Variables|Default|GetCount) (Variables|Default|GetGoodCount))
    (Rendering|SetVisibility _pointlight true false)
    (else
      (Rendering|SetVisibility _pointlight false false)))
  (return))