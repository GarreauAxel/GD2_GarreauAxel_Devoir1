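; Parent Blueprint for a swinging door that toggles open and closed, optionally opening at BeginPlay.
; A Timeline scaled by OpenAngle drives yaw, playing forward or in reverse based on ItsOpen.
; Opening sends a don't-open message through BPI_doors to linked Doors, and a timed Locker flag prevents spamming.
; When the swing finishes, it flips ItsOpen and sends add-one or less-one messages to linked lights through BPI_Light2.
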(event Custom|Opening
  ;[1 1 1] Ouverture de la porte + envois d'info a la lampe + envois d'interdiction aux autres portes de s'ouvrir pendant qu'une autre est en train de s'ouvrir
  (if (Variables|Default|Getlocker)
    (Variables|Default|Setlocker false)
    (for _array_element (Variables|Default|GetDoors)
      (if (Utilities|DoesObjectImplementInterface _array_element "/Game/Items/Blueprint/BPI_doors.BPI_doors_C")
        (Class|BPIDoors|Don'tOpen(Message) _array_element)
        (if (Variables|Default|GetItsOpen)
          (bind _newtrack_0 (Timeline|Timeline Reverse)
            (:Update
              (Transformation|SetActorRotation (Math|Rotator|MakeRotator 0.0 0.0 (* _newtrack_0 (Variables|Default|GetOpenAngle)))))
            (:Finished
              (Variables|Default|Setlocker true)
              (if (Variables|Default|GetItsOpen)
                (Variables|Default|SetItsOpen false)
                (else
                  (Variables|Default|SetItsOpen true)))
              (for _array_element_2 (Variables|Default|GetActor)
                (if (Utilities|DoesObjectImplementInterface _array_element_2 "/Game/Items/Blueprint/BPI_Light2.BPI_Light2_C")
                  (if (Variables|Default|GetItsOpen)
                    (Class|BPILight2|AddOne(Message) _array_element_2)
                    (else
                      (Class|BPILight2|LessOne(Message) _array_element_2)))))))
          (else
            (Timeline|Timeline PlayFromStart)))))))

(event EventBeginPlay
  ;[1 1 1] Tout simplement savoir si la porte doit s'ouvrir des le début
  (CallFunction|DoYoubeOpen))

(event Collision|EventActorBeginOverlap
  (params (OtherActor :type Actor%20Object%20Reference)))

(event EventTick
  (params (DeltaSeconds :type Float%20%28single-precision%29)))

(event EventToOpen
  (CallFunction|Opening))

(event EventDon'tOpen
  ;[1 1 1] Permet de ne pas pouvoir spammer l'ouverture des portes
  (Utilities|FlowControl|Delay 0.2)
  (Variables|Default|Setlocker false)
  (Utilities|FlowControl|Delay 0.8)
  (Variables|Default|Setlocker true))

(fn ConstructionScript)

(fn DoYoubeOpen
  (if (Variables|Default|GetOpenAtStart)
    (CallFunction|Opening)))