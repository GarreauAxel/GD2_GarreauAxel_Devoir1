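; BP_Door is an interactable door actor that swings open and closed when activated.
; Activate calls Opening, which waits for a delay, prints a debug string, then plays the Timeline from start or reverses it based on ItsOpen.
; The Timeline sets the actor's yaw to its track value scaled by OpenAngle and toggles ItsOpen when finished.
; The Off event is empty.
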(event Custom|Opening
  (Utilities|FlowControl|Delay (Variables|Default|GetDelay))
  (Development|PrintString "opening")
  (if (Variables|Default|GetIt'sOpen)
    (bind _newtrack_0 (Timeline|Timeline Reverse)
      (:Update
        (Transformation|SetActorRotation (Math|Rotator|MakeRotator 0.0 0.0 (* _newtrack_0 (Variables|Default|GetOpenAngle)))))
      (:Finished
        (if (Variables|Default|GetIt'sOpen)
          (Variables|Default|SetIt'sOpen false)
          (else
            (Variables|Default|SetIt'sOpen true)))))
    (else
      (Timeline|Timeline PlayFromStart))))

(event EventBeginPlay)

(event Collision|EventActorBeginOverlap
  (params (OtherActor :type Actor%20Object%20Reference)))

(event EventTick
  (params (DeltaSeconds :type Float%20%28single-precision%29)))

(event EventOff)

(event EventActivate
  (CallFunction|Opening))

(fn ConstructionScript)