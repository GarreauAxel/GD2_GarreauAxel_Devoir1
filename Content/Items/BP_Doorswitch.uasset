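; BP_Doorswitch is a trigger switch that opens the BP_Door actors in the level in a staggered sequence.
; BeginPlay caches every BP_Door, and the third-person character entering the box gives each door an index-based delay before calling its Opening event.
; A separate custom event, wapiland, not called in this graph, uses a looping timer to open the first four doors one at a time, with a debug print.
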(event OnComponentBeginOverlap(Box)
  (params (OverlappedComponent :type Primitive%20Component%20Object%20Reference) (OtherActor :type Actor%20Object%20Reference) (OtherComp :type Primitive%20Component%20Object%20Reference) (OtherBodyIndex :type Integer) (bFromSweep :type Boolean) (SweepResult :type Hit%20Result%20Structure%20%28by%20ref%29))
  (Utilities|Casting|CastToBP_ThirdPersonCharacter OtherActor)
  (for (_array_element _array_index) (Variables|Default|GetBP_Door)
    (Variables|/Game/Items/BP_Door.BP_Door_C|SetDelay _array_element (/ (Math|Conversions|ToFloat(Integer) _array_index) 4.0))
    (Default|Opening _array_element)))

(event Custom|Open2
  (Development|PrintString "Hello")
  (if (not (>= (Variables|Default|GetInteger) 4))
    (Default|Opening (Utilities|Array|Get(acopy) (Variables|Default|GetBP_Door) (Variables|Default|GetInteger)))
    (Variables|Default|SetInteger (+ (Variables|Default|GetInteger) 1))))

(event Custom|wapiland
  (Utilities|Time|SetTimerbyEvent (delegate Custom|Open2) 0.5 true))

(event EventBeginPlay
  (bind _outactors (Actor|GetAllActorsOfClass "/Game/Items/BP_Door.BP_Door_C"))
  (Variables|Default|SetBP_Door _outactors))

(event Collision|EventActorBeginOverlap
  (params (OtherActor :type Actor%20Object%20Reference)))

(event EventTick
  (params (DeltaSeconds :type Float%20%28single-precision%29)))

(fn ConstructionScript)