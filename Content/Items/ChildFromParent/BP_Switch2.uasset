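; BP_Switch2 is an interactable switch item that signals linked doors.
; Its Interaction event prints a debug "Hello", then calls the opening event.
; That event loops over the Actor array and sends YesMessage to each entry implementing the BPI_doors interface, so the switch needs no cast to specific door classes.
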(event Custom|opening
  (for _array_element (Variables|Default|Getactor)
    (if (Utilities|DoesObjectImplementInterface _array_element "/Game/Items/Blueprint/BPI_doors.BPI_doors_C")
      (Class|BPIDoors|Yes(Message) _array_element))))

(event EventBeginPlay
  (|CallParentFunction) ; This node is disabled and will not be called.\nDrag off pins to build functionality.
)

(event Collision|EventActorBeginOverlap
  (params (OtherActor :type Actor%20Object%20Reference))
  (|CallParentFunction OtherActor) ; This node is disabled and will not be called.\nDrag off pins to build functionality.
)

(event EventTick
  (params (DeltaSeconds :type Float%20%28single-precision%29))
  (|CallParentFunction DeltaSeconds) ; This node is disabled and will not be called.\nDrag off pins to build functionality.
)

(event EventInteraction
  (Development|PrintString "Hello")
  (CallFunction|Opening))

(fn ConstructionScript
  (|CallParentFunction))