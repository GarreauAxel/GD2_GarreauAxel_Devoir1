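; BP_SwichParent is a parent switch actor that opens linked doors once a main switch authorizes it.
; The Youcan event sets the Locker flag and reveals a point light to show the switch is usable.
; Interaction prints a debug string, then, if unlocked, calls Opening, which sends ToOpenMessage to each referenced actor implementing the BPI_doors interface.
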(event Custom|opening
  ;[1 1 1] Dire aux portes de s'ouvrir
  (for _array_element (Variables|Default|Getactor)
    (if (Utilities|DoesObjectImplementInterface _array_element "/Game/Items/Blueprint/BPI_doors.BPI_doors_C")
      (Class|BPIDoors|ToOpen(Message) _array_element))))

(event EventBeginPlay
  (|CallParentFunction) ; This node is disabled and will not be called.\nDrag off pins to build functionality.
)

(event Collision|EventActorBeginOverlap
  (params (OtherActor :type Actor%20Object%20Reference))
  (|CallParentFunction OtherActor) ; This node is disabled and will not be called.\nDrag off pins to build functionality.
)

(event EventTick
  (params (DeltaSeconds :type Float%20%28single-precision%29))
  (|CallParentFunction DeltaSeconds) ; This node is disabled and will not be called.\nDrag off pins to build functionality.
)

(event EventInteraction
  (Development|PrintString "Hello")
  (if (Variables|Default|GetLocker)
    (CallFunction|Opening)))

(event EventYoucan
  ;[1 1 1] Attendre l'autorisation de l'interrupteur principal pour pouvoir interragir
  (Variables|Default|SetLocker true)
  (Rendering|SetVisibility (Variables|Default|GetPointLight) true false))

(fn ConstructionScript
  (|CallParentFunction))